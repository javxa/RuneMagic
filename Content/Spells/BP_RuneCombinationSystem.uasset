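; Rune combination registry that maps combinations of runes to the spells they produce.
; On BeginPlay it scans the Asset Registry for DA_RuneCombination data assets and stores each spell in the AllSpells map under its combination key.
; Invalid rune tags and duplicate keys are skipped with on-screen errors, while successful entries are also printed.
; GetCombinationSpell, the lookup by element, effect and range, is still an empty stub.
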(event EventBeginPlay
  (CallFunction|LoadAllSpells))

(event Collision|EventActorBeginOverlap
  (params (OtherActor :type Actor%20Object%20Reference)))

(event EventTick
  (params (DeltaSeconds :type Float%20%28single-precision%29)))

(fn ConstructionScript)

(fn GetCombinationSpell
  (params (Element :type Rune%20Type%20Element%20Object%20Reference) (Effect :type Rune%20Type%20Effect%20Object%20Reference) (Range :type Rune%20Type%20Range%20Object%20Reference))
  (return 0))

(fn LoadAllSpells
  (bind _outassetdata (Class|AssetRegistry|GetAssetsbyClass (Class|AssetRegistryHelpers|GetAssetRegistry) (Class|KismetSystemLibrary|GetClassTopLevelAssetPath "/Game/Spells/DA_RuneCombination.DA_RuneCombination_C") false))
  (for _array_element _outassetdata
    (bind _asda_rune_combination (Utilities|Casting|CastToDA_RuneCombination (Class|AssetRegistryHelpers|GetAsset _array_element)))
    (bind _key (CallFunction|GetCombinationKey _asda_rune_combination))
    (if (Utilities|String|Contains (Utilities|String|ToString(Name) _key) "INVALID")
      (Development|PrintString (Utilities|String|Append "Combination " (Utilities|GetDisplayName _asda_rune_combination) " is built by runes with invalid tag(s): " (Utilities|String|ToString(Name) _key)) true true "(R=1.000000,G=0.000000,B=0.006678,A=1.000000)" 2e+01)
      (elif (.ReturnValue (Utilities|Map|Find (Variables|Default|GetAllSpells) _key))
        (Development|PrintString (Utilities|String|Append "Combination " (Utilities|GetDisplayName _asda_rune_combination) " is built by the same runes as: " (Utilities|GetClassDisplayName (.Value (Utilities|Map|Find (Variables|Default|GetAllSpells) _key)))) true true "(R=1.000000,G=0.000000,B=0.013939,A=1.000000)" 2e+01)
        (else
          (Utilities|Map|Add (Variables|Default|GetAllSpells) _key (Variables|/Game/Spells/DA_RuneCombination.DA_RuneCombination_C|GetSpell _asda_rune_combination))
          (Development|PrintString (Utilities|String|Append "Found spell: " (Utilities|GetDisplayName _asda_rune_combination) " with key: " (Utilities|String|ToString(Name) _key)) true true "(R=0.136643,G=1.000000,B=0.000000,A=1.000000)" 1e+01))))))