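; Blueprint function library that builds lookup keys for spell combinations of element, effect and range.
; GetCombinationKey breaks a combination struct into its three parts and passes them to GetCombinationKeyParts.
; That function joins each part's namespaced key with dots and returns the result as a Name.
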(fn GetCombinationKey
  (params (Combination :type DA%20Rune%20Combination%20Object%20Reference))
  (bind _key (CallFunction|GetCombinationKey(Parts) (Variables|/Game/Spells/DA_RuneCombination.DA_RuneCombination_C|GetElement Combination) (Variables|/Game/Spells/DA_RuneCombination.DA_RuneCombination_C|GetEffect Combination) (Variables|/Game/Spells/DA_RuneCombination.DA_RuneCombination_C|GetRange Combination)))
  (return _key))

(fn GetCombinationKey(Parts)
  (params (Element :type Rune%20Type%20Element%20Object%20Reference) (Effect :type Rune%20Type%20Effect%20Object%20Reference) (Range :type Rune%20Type%20Range%20Object%20Reference))
  (return (Utilities|String|StringToName (Utilities|String|Append (Utilities|String|ToString(Name) (Variables|/Game/Rune/RuneType.RuneType_C|GetNamespaced%20Key Element)) "." (Utilities|String|ToString(Name) (Variables|/Game/Rune/RuneType.RuneType_C|GetNamespaced%20Key Effect)) "." (Utilities|String|ToString(Name) (Variables|/Game/Rune/RuneType.RuneType_C|GetNamespaced%20Key Range))))))