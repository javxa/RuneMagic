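; BP_FilteredItemContainer is a factory item container that restricts which items it accepts by class.
; AcceptsItem returns true when the item's class is a child of any class in ItemFilter, printing debug strings as it checks.
; GetStackSize overrides the parent's result with MaxStackSize when UseMaxStackSize is set, and otherwise defers to the parent.
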(fn AcceptsItem
  (params (Item :type Item%20Object%20Reference))
  (for _array_element (Variables|Inventory|GetItemFilter)
    (Development|PrintString (Utilities|String|ToString(Boolean) (Utilities|ClassIsChildOf (Utilities|GetClass Item) _array_element)))
    (if (Utilities|ClassIsChildOf (Utilities|GetClass Item) _array_element)
      (return true)))
  (Development|PrintString "Complete")
  (return false))

(fn GetStackSize
  (params (Item :type Item%20Object%20Reference))
  (if (Variables|Inventory|GetUse%20Max%20Stack%20Size)
    (return (Variables|Inventory|GetMax%20Stack%20Size))
    (else
      (return (|CallParentFunction Item)))))