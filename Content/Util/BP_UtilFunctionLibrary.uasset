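; BP_UtilFunctionLibrary is a utility function library with helpers for inventory identity checks and nearest-actor lookup.
; HasInventoryEquals casts both inventory references to Object and compares them, returning false if either cast fails.
; GetClosestActor linearly scans an actor array using squared distances to a world location, then returns the nearest actor and its square-rooted distance.
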(fn HasInventoryEquals
  (params (Inventory%201 :type BPI%20Has%20Inventory%20Interface) (Inventory%202 :type BPI%20Has%20Inventory%20Interface))
  (bind _asobject (Utilities|Casting|CastToObject Inventory%201)
    (:then
      (bind _asobject_2 (Utilities|Casting|CastToObject Inventory%202)
        (:then
          (return (== _asobject _asobject_2)))
        (:CastFailed
          _)))
    (:CastFailed
      _))
  (return false))

(fn GetClosestActor
  (params (Actors :type Array%20of%20Actor%20Object%20References) (World%20Location :type Vector))
  (for (_array_element _array_index) Actors
    (if (== _array_index 0)
      (LocalVariables|SetMin%20Distance (Class|KismetMathLibrary|VectorDistanceSquared (Transformation|GetActorLocation _array_element) World%20Location))
      (LocalVariables|SetMin%20Actor _array_element)
      (elif (< (Class|KismetMathLibrary|VectorDistanceSquared (Transformation|GetActorLocation _array_element) World%20Location) (LocalVariables|GetMin%20Distance))
        (LocalVariables|SetMin%20Distance (Class|KismetMathLibrary|VectorDistanceSquared (Transformation|GetActorLocation _array_element) World%20Location))
        (LocalVariables|SetMin%20Actor _array_element))))
  (return (LocalVariables|GetMin%20Actor) (Math|Float|Sqrt (LocalVariables|GetMin%20Distance))))